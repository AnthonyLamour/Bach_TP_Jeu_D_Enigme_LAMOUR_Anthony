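; Timer actor that shows a minutes:seconds countdown on its MonText text render component and quits the game when time runs out.
; BeginPlay runs a self-looping one-second Delay that decrements NbSeconde, rolls over into NbMinute, and zero-pads seconds before updating the text.
; The construction script applies the Color variable to the text.
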(event `self.ReceiveBeginPlay`
  (`KismetSystemLibrary.Delay` 1.0 :!label _label)
  (set `self.NbSeconde` (- (`self.NbSeconde`) 1))
  (if (== (`self.NbSeconde`) -1)
    (set `self.NbSeconde` 59)
    (set `self.NbMinute` (- (`self.NbMinute`) 1))
    (if (== (`self.NbMinute`) -1)
      (`KismetSystemLibrary.QuitGame` null "Quit")
      (else
        (if (>= (`self.NbSeconde`) 10) :!label _label_2
          (set `self.Aff` (`KismetStringLibrary.Concat_StrStr` (`KismetStringLibrary.Concat_StrStr` (`KismetStringLibrary.Conv_IntToString` (`self.NbMinute`)) ":") (`KismetStringLibrary.Conv_IntToString` (`self.NbSeconde`))))
          (else
            (set `self.Aff` (`KismetStringLibrary.Concat_StrStr` (`KismetStringLibrary.Concat_StrStr` (`KismetStringLibrary.Conv_IntToString` (`self.NbMinute`)) ":0") (`KismetStringLibrary.Conv_IntToString` (`self.NbSeconde`))))))
        (`TextRenderComponent.K2_SetText` (`self.MonText`) (`KismetTextLibrary.Conv_StringToText` (`self.Aff`)))
        (goto _label)))
    (else
      (goto _label_2))))

(fn `UserConstructionScript`
  (`TextRenderComponent.SetTextRenderColor` (`self.MonText`) (`self.Color`)))