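; Mur_Avec_Texte is a configurable wall actor with a text label, set up entirely in its construction script.
; It scales the static mesh from MurX, MurY and MurZ and applies MurMaterial to it.
; The MonText component gets its scale, offset, color and content from variables, with world rotation derived from a direction vector via RotationFromXVector.
; The event graph holds only disabled placeholder events, so it adds no runtime logic.
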(fn `UserConstructionScript`
  (bind _staticmesh (`self.StaticMesh`))
  (bind _montext (`self.MonText`))
  (`SceneComponent.SetWorldScale3D` _staticmesh (`KismetMathLibrary.MakeVector` (`self.MurX`) (`self.MurY`) (`self.MurZ`)))
  (`SceneComponent.SetWorldScale3D` _montext (`self.TextScale`))
  (`SceneComponent.K2_AddLocalOffset` _montext (`self.TextPosition`) false false)
  (`SceneComponent.K2_SetWorldRotation` _montext (`KismetMathLibrary.Conv_VectorToRotator` (`self.TextRotation`)) false false)
  (`TextRenderComponent.K2_SetText` _montext (`KismetTextLibrary.Conv_StringToText` (`self.Text`)))
  (`TextRenderComponent.SetTextRenderColor` _montext (`self.TextColor`))
  (`PrimitiveComponent.SetMaterial` _staticmesh 0 (`self.MurMaterial`)))