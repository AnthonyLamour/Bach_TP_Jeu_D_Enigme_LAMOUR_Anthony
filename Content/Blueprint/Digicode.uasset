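; Digicode is a keypad that gates a Door behind a code entered through a UI widget.
; Using the keypad creates the BP_Code widget with a reference back to itself, then switches to UI-only input with a visible mouse cursor.
; Its correct and wrong password events forward the result to the Door, which either opens or runs its wrong-code response.
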(event `Use_Keypad`
  (bind _returnvalue (`GameplayStatics.GetPlayerController` 0))
  (bind _returnvalue_2 (`|CreateWidget` "/Game/Blueprint/BP_Code.BP_Code_C"))
  (set `/Game/Blueprint/BP_Code.SecurityCode` self _returnvalue_2)
  (`UserWidget.AddToViewport` _returnvalue_2 0)
  (`WidgetBlueprintLibrary.SetInputMode_UIOnlyEx` _returnvalue _returnvalue_2)
  (set `PlayerController.bShowMouseCursor` true _returnvalue))

(event `Correct_Password`
  (`/Game/Blueprint/BP_Door.OpenDoor` (`self.Door`)))

(event `WrongPassword`
  (`/Game/Blueprint/BP_Door.WrongCode` (`self.Door`)))

(fn `UserConstructionScript`)