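; Player pawn with axis-driven look and movement that plays music on BeginPlay and quits the game on Escape.
; Movement follows only the controller's yaw, so looking up or down does not affect its direction.
; Pressing F sphere-traces a short distance from the eye viewpoint and calls UseKeypad on a hit Digicode actor, printing a debug string for other hits.
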(event `InputAxis|Look_Left_Right`
  (params (AxisValue :type "Float (single-precision)"))
  ;[1 1 1] Look
  (`self.AddControllerYawInput` AxisValue))

(event `Key|Escape`
  (params (Key :type "Key Structure"))
  (:`Pressed`
    (`KismetSystemLibrary.QuitGame` null "Quit")))

(event `InputAxis|Look_Up_Down`
  (params (AxisValue :type "Float (single-precision)"))
  ;[1 1 1] Look
  (`self.AddControllerPitchInput` AxisValue))

(event `InputAxis|Move_Forward_Backward`
  (params (AxisValue :type "Float (single-precision)"))
  (bind _returnvalue (`GameplayStatics.GetPlayerController` 0))
  (bind (_returnvalue_roll _returnvalue_pitch _returnvalue_yaw) (`KismetMathLibrary.BreakRotator` (`Controller.GetControlRotation` _returnvalue)))
  ;[1 1 1] Move
  (`self.AddMovementInput` (`Controller.K2_GetPawn` _returnvalue) (`KismetMathLibrary.GetForwardVector` (`KismetMathLibrary.MakeRotator` 0.0 0.0 _returnvalue_yaw)) AxisValue false))

(event `self.ReceiveBeginPlay`
  (`AudioComponent.Play` (`self.Music`) 0.0))

(event `InputAxis|Move_Left_Right`
  (params (AxisValue :type "Float (single-precision)"))
  (bind _returnvalue (`GameplayStatics.GetPlayerController` 0))
  (bind (_returnvalue_roll _returnvalue_pitch _returnvalue_yaw) (`KismetMathLibrary.BreakRotator` (`Controller.GetControlRotation` _returnvalue)))
  ;[1 1 1] Move
  (`self.AddMovementInput` (`Controller.K2_GetPawn` _returnvalue) (`KismetMathLibrary.GetRightVector` (`KismetMathLibrary.MakeRotator` 0.0 0.0 _returnvalue_yaw)) AxisValue false))

(event `Key|F`
  (params (Key :type "Key Structure"))
  (bind (_outlocation _outrotation) (`self.GetActorEyesViewPoint` self))
  ;[1 1 1] UseDigicode
  (:`Pressed`
    (bind (_outhit _returnvalue) (`KismetSystemLibrary.SphereTraceSingle` _outlocation (+ _outlocation (* (`KismetMathLibrary.GetForwardVector` _outrotation) 400.0)) 0.0 "TraceTypeQuery1"))
    (if _returnvalue
      (bind (_bblockinghit _binitialoverlap _time _distance _location _impactpoint _normal _impactnormal _physmat _hitactor) (`GameplayStatics.BreakHitResult` _outhit))
      (if (== (`GameplayStatics.GetObjectClass` _hitactor) "/Game/Blueprint/Digicode.Digicode_C")
        (bind _asdigicode (cast `/Game/Blueprint/Digicode` _hitactor))
        (bind _output_get (set `self.Code` _asdigicode))
        (`/Game/Blueprint/Digicode.Use_Keypad` _output_get)
        (else
          (`KismetSystemLibrary.PrintString` "oups"))))))

(fn `UserConstructionScript`)