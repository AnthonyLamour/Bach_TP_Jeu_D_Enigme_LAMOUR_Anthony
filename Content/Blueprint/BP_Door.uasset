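; Door actor that swings open or signals a wrong code through two custom events.
; OpenDoor snaps the static mesh to a fixed absolute world rotation, with no animation, and plays an opening sound.
; WrongCode plays an error sound on the same audio component and leaves the mesh untouched.
; The Blueprint holds no code-checking or closing logic.
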(event `OpenDoor`
  (`SceneComponent.K2_SetWorldRotation` (`self.StaticMeshComponent`) (struct :`Yaw` 90.0) false false)
  (`AudioComponent.SetSound` (`self.Audio`) "/Game/Audio/open_door.open_door")
  (`AudioComponent.Play` (`self.Audio`) 0.0))

(event `WrongCode`
  (`AudioComponent.SetSound` (`self.Audio`) "/Game/Audio/Wrong.Wrong")
  (`AudioComponent.Play` (`self.Audio`) 0.0))

(fn `UserConstructionScript`)